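; Snow trail capture actor that records depth into a persistent render target and passes it to a landscape streaming proxy's material.
; A scene capture with an M_Depth post-process fills DrawTarget, which M_DrawPersistance draws into the persistent target each tick, offset by actor movement.
; Movement uses a pixel-grid snap helper, though its player inputs are zero and its math is unwired.
; A debug widget displays both targets.
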(event EventBeginPlay
  (Utilities|FlowControl|Sequence
    (:then_0
      (bind _returnvalue (Rendering|Material|GetScalarParameterValue "/Game/Snowball/SnowTrail/MPC_SnowTrail.MPC_SnowTrail" "CaptureSize" :!class /Script/Engine.KismetMaterialLibrary))
      (Variables|/Script/Engine.SceneCaptureComponent2D|SetOrthoWidth (Variables|Default|GetSceneCaptureComponent2D) _returnvalue)
      (CallFunction|InitializeMaterials)
      (CallFunction|InitializeTargets))
    (:then_1
      (bind _returnvalue_2 (Actor|GetActorOfClass "/Script/Landscape.LandscapeStreamingProxy"))
      (Development|PrintString (Utilities|GetDisplayName _returnvalue_2))
      (Landscape|Runtime|Material|SetLandscapeMaterialTextureParameterValue _returnvalue_2 "DepthTarget" (Variables|Default|GetPersistentDepthTarget)))
    (:then_2
      ;[1 1 1] Reset to default height
      (Rendering|ClearRenderTarget2D (Variables|Default|GetPersistentDepthTarget))
      (Rendering|ClearRenderTarget2D (Variables|Default|GetDrawTarget)))
    (:then_3
      (bind _returnvalue_3 (UserInterface|CreateWidget "/Game/Snowball/UI/WBP_RenderTarget.WBP_RenderTarget_C" (Game|GetPlayerController 0)))
      (UserInterface|Viewport|AddtoViewport _returnvalue_3 0)
      (Default|Update _returnvalue_3 (Variables|Default|GetDrawTarget) (Variables|Default|GetPersistentDepthTarget)))))

(event EventTick
  (params (DeltaSeconds :type Float%20%28single-precision%29))
  (Utilities|FlowControl|Sequence
    (:then_0
      (CallFunction|SetLocationtoPlayer))
    (:then_1
      (CallFunction|UpdateCaptureLocationVectorParameter))
    (:then_2
      ;[1 1 1] Draw to Persistent
      (CallFunction|SetMaterialOffset))
    (:then_3
      (CallFunction|SavetoPersistent))
    (:then_4
      (Default|Update (stale EventBeginPlay _returnvalue_3) (Variables|Default|GetDrawTarget) (Variables|Default|GetPersistentDepthTarget)))))

(fn ConstructionScript
  ;[1 1 1] Sets default capture size from parameters
)

(fn SetLocationtoPlayer
  (bind _returnvalue (Transformation|GetActorLocation))
  (bind _returnvalue_2 (/ 1.0 256.0))
  (bind _scenecapturecomponent2d (Variables|Default|GetSceneCaptureComponent2D))
  (bind _orthowidth (Variables|/Script/Engine.SceneCaptureComponent2D|GetOrthoWidth _scenecapturecomponent2d))
  (bind _returnvalue_3 (* _orthowidth _returnvalue_2))
  (bind _returnvalue_4 (Utilities|SnapPixeltoGrid 0.0 0.0 _returnvalue_3))
  (bind _returnvalue_5 (- _returnvalue_4 _returnvalue))
  (bind _output_get (Variables|Default|SetMoveOffset (Math|Vector2D|MakeVector2D (.x _returnvalue_5) (.y _returnvalue_5))))
  (Transformation|AddActorWorldOffset (Math|Vector|MakeVector (.x _output_get) (.y _output_get) 0.0)))

(fn UpdateCaptureLocationVectorParameter
  (Rendering|Material|SetVectorParameterValue "/Game/Snowball/SnowTrail/MPC_SnowTrail.MPC_SnowTrail" "CaptureLocation" (Math|Conversions|ToLinearColor(Vector) (Transformation|GetActorLocation)) :!class /Script/Engine.KismetMaterialLibrary))

(fn SetMaterialOffset
  (bind _moveoffset (Variables|Default|GetMoveOffset))
  (bind _scenecapturecomponent2d (Variables|Default|GetSceneCaptureComponent2D))
  (bind _orthowidth (Variables|/Script/Engine.SceneCaptureComponent2D|GetOrthoWidth _scenecapturecomponent2d))
  (bind _returnvalue (/ _moveoffset _orthowidth))
  ;[1 1 1] See this is material Offset being set
  (Rendering|Material|SetVectorParameterValue (Variables|Default|GetDrawMaterial) "Offset" (Utilities|Struct|MakeLinearColor (.x _returnvalue) (.y _returnvalue) 0.0 1.0) :!class /Script/Engine.MaterialInstanceDynamic))

(fn SavetoPersistent
  (Rendering|DrawMaterialtoRenderTarget (Variables|Default|GetPersistentDepthTarget) (Variables|Default|GetDrawMaterial)))

(fn InitializeMaterials
  (Utilities|FlowControl|Sequence
    (:then_0
      (bind _returnvalue (Rendering|Material|CreateDynamicMaterialInstance "/Game/Snowball/SnowTrail/M_Depth.M_Depth" "None" "None" :!class /Script/Engine.KismetMaterialLibrary))
      (Variables|Default|SetDepthMaterial _returnvalue)
      (bind _returnvalue_2 (Rendering|CreateRenderTarget2D 256 256 "RTF_RGBA16f"))
      (Variables|Default|SetPersistentDepthTarget _returnvalue_2)
      (Rendering|Material|SetTextureParameterValue (Variables|Default|GetDepthMaterial) "PermTarget" (Variables|Default|GetPersistentDepthTarget)))
    (:then_1
      (bind _returnvalue_3 (Rendering|Material|CreateDynamicMaterialInstance "/Game/Snowball/SnowTrail/M_DrawPersistance.M_DrawPersistance" "None" "None" :!class /Script/Engine.KismetMaterialLibrary))
      (Variables|Default|SetDrawMaterial _returnvalue_3)
      (bind _returnvalue_4 (Rendering|CreateRenderTarget2D 256 256 "RTF_RGBA16f"))
      (Variables|Default|SetDrawTarget _returnvalue_4)
      (Rendering|Material|SetTextureParameterValue (Variables|Default|GetDrawMaterial) "DrawTarget" (Variables|Default|GetDrawTarget)))))

(fn InitializeTargets
  (bind _scenecapturecomponent2d (Variables|Default|GetSceneCaptureComponent2D))
  (Variables|/Script/Engine.SceneCaptureComponent2D|SetTextureTarget _scenecapturecomponent2d (Variables|Default|GetDrawTarget))
  (Variables|/Script/Engine.SceneCaptureComponent2D|SetPostProcessSettings _scenecapturecomponent2d (Utilities|Struct|MakePostProcessSettings (Utilities|Struct|MakeWeightedBlendables (Utilities|Array|MakeArray (Utilities|Struct|MakeWeightedBlendable 1.0 (Variables|Default|GetDepthMaterial)))))))