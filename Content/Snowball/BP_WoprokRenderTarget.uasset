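; Scene capture actor that follows the player and maintains a persistent render target for the Woprok snow effect.
; BeginPlay clears both render targets, publishes capture size to MPC_WoprokSnow and creates the draw material.
; Each tick it moves in XY by SnapPixelToGrid's texel-sized steps (ortho width / 256) and publishes its location to the collection.
; It then draws into the persistent target, passing the normalized move as the material's Offset.
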(event EventBeginPlay
  (Rendering|Material|SetScalarParameterValue "/Game/Snowball/MPC_WoprokSnow.MPC_WoprokSnow" "CaptureSize" (Variables|/Script/Engine.SceneCaptureComponent2D|GetOrthoWidth (Variables|Default|GetSceneCaptureComponent2D)) :!class /Script/Engine.KismetMaterialLibrary)
  (bind _returnvalue (Rendering|Material|CreateDynamicMaterialInstance "/Game/Snowball/M_WoprokDrawToPersistance.M_WoprokDrawToPersistance" "None" "None" :!class /Script/Engine.KismetMaterialLibrary))
  (Variables|Default|SetDrawToPersistentMarterial _returnvalue)
  (Rendering|ClearRenderTarget2D "/Game/Snowball/BP_WoprokTextureRenderTarget2D.BP_WoprokTextureRenderTarget2D")
  (Rendering|ClearRenderTarget2D "/Game/Snowball/BP_WoprokPersistentTextureRenderTarget2D.BP_WoprokPersistentTextureRenderTarget2D"))

(event EventTick
  (params (DeltaSeconds :type Float%20%28single-precision%29))
  (CallFunction|MoveCapture)
  (CallFunction|DrawtoPersistent))

(fn ConstructionScript)

(fn MoveCapture
  (bind _returnvalue (Game|GetPlayerCharacter 0))
  (bind _returnvalue_2 (Transformation|GetActorLocation))
  (bind _returnvalue_3 (/ 1.0 256.0))
  (bind _scenecapturecomponent2d (Variables|Default|GetSceneCaptureComponent2D))
  (bind _returnvalue_4 (Transformation|GetActorLocation _returnvalue))
  (bind _orthowidth (Variables|/Script/Engine.SceneCaptureComponent2D|GetOrthoWidth _scenecapturecomponent2d))
  (bind _returnvalue_5 (* _orthowidth _returnvalue_3))
  (bind _returnvalue_6 (Utilities|SnapPixeltoGrid (.x _returnvalue_4) (.y _returnvalue_4) _returnvalue_5))
  (bind _returnvalue_7 (- _returnvalue_6 _returnvalue_2))
  (bind _output_get (Variables|Default|SetMoveOffset (Math|Vector2D|MakeVector2D (.x _returnvalue_7) (.y _returnvalue_7))))
  (Transformation|AddActorWorldOffset (Math|Vector|MakeVector (.x _output_get) (.y _output_get) 0.0))
  (Rendering|Material|SetVectorParameterValue "/Game/Snowball/MPC_WoprokSnow.MPC_WoprokSnow" "CaptureLocation" (Math|Conversions|ToLinearColor(Vector) (Transformation|GetActorLocation)) :!class /Script/Engine.KismetMaterialLibrary))

(fn DrawtoPersistent
  (bind _moveoffset (Variables|Default|GetMoveOffset))
  (bind _scenecapturecomponent2d (Variables|Default|GetSceneCaptureComponent2D))
  (bind _orthowidth (Variables|/Script/Engine.SceneCaptureComponent2D|GetOrthoWidth _scenecapturecomponent2d))
  (bind _returnvalue (/ _moveoffset _orthowidth))
  ;[1 1 1] See this is material Offset being set
  (Rendering|Material|SetVectorParameterValue (Variables|Default|GetDrawToPersistentMarterial) "Offset" (Utilities|Struct|MakeLinearColor (.x _returnvalue) (.y _returnvalue) 0.0 1.0) :!class /Script/Engine.MaterialInstanceDynamic)
  (Rendering|DrawMaterialtoRenderTarget "/Game/Snowball/BP_WoprokPersistentTextureRenderTarget2D.BP_WoprokPersistentTextureRenderTarget2D" (Variables|Default|GetDrawToPersistentMarterial)))