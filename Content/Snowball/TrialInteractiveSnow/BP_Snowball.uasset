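; BP_Snowball is a snowball actor that grows as it moves through the world.
; Each tick it measures the distance moved since the previous frame, multiplies it by ScaleValue and adds the result to a running Scale.
; That Scale is applied uniformly as the actor's 3D scale, and the stored position is then updated, so growth follows total distance travelled.
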(event EventBeginPlay
  (Variables|Default|SetOriginalPosition (Transformation|GetActorLocation)))

(event Collision|EventActorBeginOverlap
  (params (OtherActor :type Actor%20Object%20Reference)))

(event EventTick
  (params (DeltaSeconds :type Float%20%28single-precision%29))
  (bind _output_get (Variables|Default|SetScale (+ (* (Math|Vector|VectorLength (- (Transformation|GetActorLocation) (Variables|Default|GetOriginalPosition))) (Variables|Default|GetScaleValue)) (Variables|Default|GetScale))))
  (Transformation|SetActorScale3D (Math|Conversions|ToVector(Float) _output_get))
  (Variables|Default|SetOriginalPosition (Transformation|GetActorLocation)))

(fn ConstructionScript)