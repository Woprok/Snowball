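; BP_Snowfall is a snowfall effect actor that periodically randomizes its wind.
; From BeginPlay, ChangeWind sets a random signed wind power on the NSSnowfall component through its UserWindPower variable.
; After a random delay it gives the actor a random yaw, prints a debug message and calls itself again, forming an endless timed loop.
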(event Custom|ChangeWind
  (Niagara|SetNiagaraVariable(Float) (Variables|Default|GetNS_Snowfall) (Variables|Default|GetUser_WindPower) (Math|Random|RandomFloatinRange -3e+01 3e+01))
  (Utilities|FlowControl|Delay (Math|Random|RandomFloatinRange 1e+01 2e+01))
  (Transformation|SetActorRotation (Math|Rotator|MakeRotator 0.0 0.0 (Math|Random|RandomFloatinRange 0.0 3.6e+02)))
  (Development|PrintText "Changed Wind" true true "(R=1.000000,G=0.000000,B=0.147162,A=1.000000)")
  (CallFunction|ChangeWind))

(event EventBeginPlay
  (CallFunction|ChangeWind))

(fn ConstructionScript)